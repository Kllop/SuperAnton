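; Parent Blueprint for modular Paper2D platforms that randomly spawn an enemy, a healing pickup or a shield.
; The construction script builds bottom, middle and top rows from structs of five optional segments, each a sprite with a Pawn-blocking box, and adds one overlap box.
; BeginPlay rolls each drop chance, using nested random ranges for enemy and heart, then spawns at a random tagged component and destroys that component.
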(event `self.ReceiveBeginPlay`
  (`|ExecutionSequence`
    (:`then_0`
      (if (== (`KismetMathLibrary.RandomIntegerInRange` 1 (`KismetMathLibrary.RandomIntegerInRange` 1 (`KismetMathLibrary.Round` (/ 100.0 (`self.DropChance_Enemy`))))) 1)
        (`self.SpawnElem` "/Game/Blueprints/Enemies/BaseEnemy.BaseEnemy_C" "Enemy")))
    (:`then_1`
      (if (== (`KismetMathLibrary.RandomIntegerInRange` 1 (`KismetMathLibrary.RandomIntegerInRange` 1 (`KismetMathLibrary.Round` (/ 100.0 (`self.DropChance_Heart`))))) 1)
        (`self.SpawnElem` "/Game/Blueprints/Objects/BP_Heling.BP_Heling_C" "Heart")))
    (:`then_2`
      (if (== (`KismetMathLibrary.RandomIntegerInRange` 1 (`KismetMathLibrary.Round` (/ 100.0 (`self.DropChance_Shield`)))) 1)
        (`self.SpawnElem` "/Game/Blueprints/Objects/BP_Shield.BP_Shield_C" "Shield")))))

(event `self.ReceiveTick`
  (params (DeltaSeconds :type "Float (single-precision)"))
  (set `self.Locaiton` (`self.K2_GetActorLocation`)))

(fn `add_PaperSprite`
  (params (Location :type "Vector Structure") (Sprite :type "PaperSprite Object Reference"))
  (bind _returnvalue (`AddComponent|NODE_AddPaperSpriteComponent-1` :`RelativeTransform` (`KismetMathLibrary.MakeTransform` Location (struct) (0.4 0.4 0.4))))
  (`PrimitiveComponent.SetCollisionResponseToChannel` _returnvalue "ECC_WorldDynamic" "ECR_Ignore")
  (`PaperSpriteComponent.SetSprite` _returnvalue Sprite)
  (bind _returnvalue_2 (`AddComponent|NODE_AddBoxComponent-0` :`RelativeTransform` (`KismetMathLibrary.MakeTransform` (+ Location (0.0 0.0 70.0)))))
  (`BoxComponent.SetBoxExtent` _returnvalue_2 (172.5 14.5 14.5) true)
  (`PrimitiveComponent.SetCollisionResponseToChannel` _returnvalue_2 "ECC_WorldDynamic" "ECR_Ignore")
  (`PrimitiveComponent.SetCollisionResponseToChannel` _returnvalue_2 "ECC_Pawn" "ECR_Block")
  (`SceneComponent.SetHiddenInGame` _returnvalue_2 false false)
  (return))

(fn `Build_Platform`
  (params (Struct :type "/Game/DataTables/Structs/ST_Position_Platforms Structure") (Position_Z :type "Float (double-precision)") (`Location Y` :type "Float (double-precision)"))
  (locals (L_Struct :type "/Game/DataTables/Structs/ST_Position_Platforms Structure"))
  (bind ((`Centre_52_4B26A1A04AAC6AAA4F19C2912380A98C` _centre) (`Centre_Texture_53_1B1053274C923B90A0AD7BA427AB19A7` _centre_texture)) (break `/Game/DataTables/Structs/ST_Position_Platforms` (`local.L_Struct`)))
  (bind ((`Right_54_270F55794FC997DCDE192AB966C7B32F` _right) (`Right_Texture_55_F37CE3A3448AF2B4ABE2CFA8AFC3B1DE` _right_texture)) (break `/Game/DataTables/Structs/ST_Position_Platforms` (`local.L_Struct`)))
  (bind ((`RightEnd_56_AC51441347C3E581A8FF5A9A9E625A33` _rightend) (`RightEnd_Texture_57_6B5D82ED413C9E421BD0359FFA291745` _rightend_texture)) (break `/Game/DataTables/Structs/ST_Position_Platforms` (`local.L_Struct`)))
  (bind ((`LeftEnd_48_EA407C054EEC2427DA7AEDAB3B6C67B1` _leftend) (`LeftEnd_Texture_49_690E42C74C66682E7F382A885CD86867` _leftend_texture)) (break `/Game/DataTables/Structs/ST_Position_Platforms` (`local.L_Struct`)))
  (bind ((`Left_50_49D1974346AF4E67DD9DDD97E56FF4AF` _left) (`Left_Texture_51_E9B83F5345680CD0C95169B8D0448BD1` _left_texture)) (break `/Game/DataTables/Structs/ST_Position_Platforms` (`local.L_Struct`)))
  (set `local.L_Struct` Struct)
  (if _leftend
    (`self.add_PaperSprite` (`KismetMathLibrary.MakeVector` 0.0 `Location Y` Position_Z) _leftend_texture))
  (if _left
    (`self.add_PaperSprite` (`KismetMathLibrary.MakeVector` (`self.Step_Size_X`) `Location Y` Position_Z) _left_texture))
  (if _centre
    (`self.add_PaperSprite` (`KismetMathLibrary.MakeVector` (* (`self.Step_Size_X`) 2.0) `Location Y` Position_Z) _centre_texture))
  (if _right
    (`self.add_PaperSprite` (`KismetMathLibrary.MakeVector` (* (`self.Step_Size_X`) 3.0) `Location Y` Position_Z) _right_texture))
  (if _rightend
    (`self.add_PaperSprite` (`KismetMathLibrary.MakeVector` (* (`self.Step_Size_X`) 4.0) `Location Y` Position_Z) _rightend_texture))
  (return))

(fn `GetRandomElem`
  (params (Array :type "Array of SceneComponent Object Reference"))
  (returns (Output :type "SceneComponent Object Reference"))
  (return (`|GetArrayItem` Array (`KismetMathLibrary.RandomIntegerInRange` 0 (- (`KismetArrayLibrary.Array_Length` Array) 1)))))

(fn `Set_Collision_Box`
  (params (Struct :type "/Game/DataTables/Structs/ST_Position_Platforms Structure")))

(fn `SpawnElem`
  (params (Class :type "Actor Class Reference") (Tag :type Name))
  (bind _output (`self.GetRandomElem` (`self.GetComponentsByTag` "/Script/Engine.SceneComponent" Tag)))
  (`/Engine/EditorBlueprintResources/StandardMacros.IsValid` _output
    (:`Is Valid`
      (`|SpawnActorFromClass` Class (`KismetMathLibrary.MakeTransform` (`SceneComponent.K2_GetComponentLocation` _output)) "AlwaysSpawn" "OverrideRootScale" null null)
      (`ActorComponent.K2_DestroyComponent` _output)
      (return))))

(fn `UserConstructionScript`
  (`self.Build_Platform` (`self.Build_Buttom`))
  (`self.Build_Platform` (`self.Build_Middle`) (`self.Step_Size_Z`) (`self.Step_Size_Y`))
  (`self.Build_Platform` (`self.Build_Top`) (* (`self.Step_Size_Z`) 2.0) (* (`self.Step_Size_Y`) 2.0))
  (bind _returnvalue (`AddComponent|NODE_AddBoxComponent-1` :`RelativeTransform` (`KismetMathLibrary.MakeTransform` (1530.0 0.0 0.0))))
  (`PrimitiveComponent.SetCollisionResponseToAllChannels` _returnvalue "ECR_Ignore")
  (`PrimitiveComponent.SetCollisionResponseToChannel` _returnvalue "ECC_WorldDynamic" "ECR_Overlap"))
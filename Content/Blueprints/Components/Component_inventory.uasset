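; Inventory component that stores items as STStoreUnit structs and prints a Money value every tick.
; AddItem merges stackable items into the entry with the same name, found through FindItem's linear search, or appends a new entry.
; RemoveItem lowers stack counts by the passed struct's Count or removes non-stackable entries, returning true when nothing matches.
; A depleted stack removes index 0 instead of the found index, and the Count parameter is unused.
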(event `self.ReceiveTick`
  (params (DeltaSeconds :type "Float (single-precision)"))
  (`KismetSystemLibrary.PrintString` (`KismetStringLibrary.Conv_IntToString` (`self.Money`)) true true (struct :`G` 0.66 :`B` 1.0 :`A` 1.0) 0.0))

(fn `Add_item`
  (params (Item :type "/Game/DataTables/Structs/ST_StoreUnit Structure"))
  (locals (L_item :type "/Game/DataTables/Structs/ST_StoreUnit Structure"))
  (bind _inventory (`self.Inventory`))
  (bind _output_get (set `local.L_item` Item))
  (if (`.Stack_15_E18C33CA4AF18C5F786407924F3E6571` (break `/Game/DataTables/Structs/ST_StoreUnit` _output_get))
    (bind (_resault _index) (`self.Find_Item` (`local.L_item`)))
    (if _resault
      (bind (_name _description _texture _staticmesh _actor _stack _price _count) (break `/Game/DataTables/Structs/ST_StoreUnit` (`|GetArrayItem` _inventory _index)))
      (`KismetArrayLibrary.Array_Set` _inventory _index (make `/Game/DataTables/Structs/ST_StoreUnit` _name _description _texture _staticmesh _actor _stack _price (+ _count (`.Count_17_8C3868D04954149B9A11C5B71C8AD341` (break `/Game/DataTables/Structs/ST_StoreUnit` (`local.L_item`))))) true)
      (else
        (`KismetArrayLibrary.Array_Add` (`self.Inventory`) (`local.L_item`))))
    (else
      (`KismetArrayLibrary.Array_Add` (`self.Inventory`) (`local.L_item`)))))

(fn `Find_Item`
  (params (item :type "/Game/DataTables/Structs/ST_StoreUnit Structure"))
  (returns (Resault :type Boolean) (Index :type Integer))
  (for (_array_element _array_index) (`self.Inventory`)
    (if (== (`.Name_25_61A057AE47E9D02095F92F9F1B5B0B3B` (break `/Game/DataTables/Structs/ST_StoreUnit` _array_element)) (`.Name_25_61A057AE47E9D02095F92F9F1B5B0B3B` (break `/Game/DataTables/Structs/ST_StoreUnit` item)))
      (return true _array_index)))
  (return false 0))

(fn `Remove_item`
  (params (Name :type "/Game/DataTables/Structs/ST_StoreUnit Structure") (Count :type Integer))
  (returns (Error :type Boolean))
  (locals (L_item :type "/Game/DataTables/Structs/ST_StoreUnit Structure") (L_index :type Integer))
  (bind (_name _description _texture _staticmesh _actor _stack _price _count) (break `/Game/DataTables/Structs/ST_StoreUnit` (`|GetArrayItem` (`self.Inventory`) (`local.L_index`))))
  (bind _output_get (set `local.L_item` Name))
  (bind (_resault _index) (`self.Find_Item` _output_get))
  (if _resault
    (set `local.L_index` _index)
    (if (`.Stack_15_E18C33CA4AF18C5F786407924F3E6571` (break `/Game/DataTables/Structs/ST_StoreUnit` (`local.L_item`)))
      (if (<= (- (`.Count_17_8C3868D04954149B9A11C5B71C8AD341` (break `/Game/DataTables/Structs/ST_StoreUnit` (`|GetArrayItem` (`self.Inventory`) (`local.L_index`)))) (`.Count_17_8C3868D04954149B9A11C5B71C8AD341` (break `/Game/DataTables/Structs/ST_StoreUnit` (`local.L_item`)))) 0)
        (`KismetArrayLibrary.Array_Remove` (`self.Inventory`))
        (return false)
        (else
          (`KismetArrayLibrary.Array_Set` (`self.Inventory`) (`local.L_index`) (make `/Game/DataTables/Structs/ST_StoreUnit` _name _description _texture _staticmesh _actor _stack _price (- _count (`.Count_17_8C3868D04954149B9A11C5B71C8AD341` (break `/Game/DataTables/Structs/ST_StoreUnit` (`local.L_item`))))) true)
          (return false)))
      (else
        (`KismetArrayLibrary.Array_Remove` (`self.Inventory`) (`local.L_index`))))
    (else
      (return true))))
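; Player controller for a 2D side-scroller that handles camera changes and a scripted character move.
; BeginPlay views through the second CameraActor found by class.
; Set_Camera_2 blends to the first, sets the game mode's Run flag, and starts timers for its delayed HUD change and looping boss-spawn call.
; StartMoveCharacter uses a timeline to push the character along +X at a speed derived from its starting X position.
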(event `self.ReceiveBeginPlay`
  (bind _outactors (`GameplayStatics.GetAllActorsOfClass` "/Script/Engine.CameraActor"))
  (`self.SetViewTargetWithBlend` (`|GetArrayItem` _outactors 1)))

(event `Set_Camera_2`
  (bind _outactors (`GameplayStatics.GetAllActorsOfClass` "/Script/Engine.CameraActor"))
  (`self.SetViewTargetWithBlend` (`|GetArrayItem` _outactors) 3.0 "VTBlend_Cubic")
  (bind _as2dside_scroller_game_mode (cast `/Game/Blueprints/GameModes/2DSideScrollerGameMode` (`GameplayStatics.GetGameMode`)))
  (`KismetSystemLibrary.K2_SetTimer` _as2dside_scroller_game_mode "SetNewHUd" 3.5)
  (set `/Game/Blueprints/GameModes/2DSideScrollerGameMode.bRun` true _as2dside_scroller_game_mode)
  (`KismetSystemLibrary.K2_SetTimer` _as2dside_scroller_game_mode "SpawnBoss" 1.0 true))

(event `StartMoveCharacter`
  (bind _returnvalue (`GameplayStatics.GetActorOfClass` "/Game/Blueprints/Characters/2DSideScrollerCharacter.2DSideScrollerCharacter_C"))
  (set `self.Lenght` (`KismetMathLibrary.Abs` (+ (.x (`self.K2_GetActorLocation` _returnvalue)) 700.0)))
  (`Timeline|Timeline_0` :!via `PlayFromStart`
    (:`Update`
      (`self.K2_AddActorWorldOffset` _returnvalue (`KismetMathLibrary.MakeVector` (* (/ (`self.Lenght`) 2.0) (`GameplayStatics.GetWorldDeltaSeconds`))) false false))))

(fn `UserConstructionScript`)
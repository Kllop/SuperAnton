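; BP_SpawnPlatform is a trigger-box actor that spawns a follow-on BP_TEST, apparently a platform segment, for a side-scroller.
; When a BP_TEST stops overlapping the box, it spawns another at that actor's location, offset along X by its StepSize.
; The new actor is appended to ArrayPlatforms on the 2DSideScrollerGameMode.
; The construction script sizes the box from SizeBox.
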(event `self.Box.OnComponentEndOverlap`
  (params (OverlappedComponent :type "PrimitiveComponent Object Reference") (OtherActor :type "Actor Object Reference") (OtherComp :type "PrimitiveComponent Object Reference") (OtherBodyIndex :type Integer))
  (bind _asbp_test (cast `/Game/Blueprints/Objects/BP_TEST` OtherActor))
  (bind _returnvalue (`|SpawnActorFromClass` "/Game/Blueprints/Objects/BP_TEST.BP_TEST_C" (`KismetMathLibrary.MakeTransform` (+ (`/Game/Blueprints/Objects/BP_TEST.ActorLocation` _asbp_test) (`KismetMathLibrary.MakeVector` (`/Game/Blueprints/Objects/BP_TEST.StepSize` _asbp_test))) (struct) (1.0 1.0 1.0)) "AdjustIfPossibleButAlwaysSpawn" "OverrideRootScale" null null))
  (bind _as2dside_scroller_game_mode (cast `/Game/Blueprints/GameModes/2DSideScrollerGameMode` (`GameplayStatics.GetGameMode`)))
  (`KismetArrayLibrary.Array_Add` (`/Game/Blueprints/GameModes/2DSideScrollerGameMode.ArrayPlatforms` _as2dside_scroller_game_mode) _returnvalue))

(fn `UserConstructionScript`
  (`BoxComponent.SetBoxExtent` (`self.Box`) (`self.SizeBox`) true))
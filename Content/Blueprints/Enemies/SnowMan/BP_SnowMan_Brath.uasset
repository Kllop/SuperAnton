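; BP_SnowMan_Brath is a flipbook actor, apparently the snowman enemy's breath effect.
; BeginPlay starts a one-shot timer lasting the length of its PaperFlipbook animation.
; DestroySelf destroys the actor, while RemoveFB, despite its name, replays the Brath flipbook from the start.
; Unconnected construction-script nodes hold an unused setup that adds attack and breath flipbook components with a looping timer.
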(event `self.ReceiveBeginPlay`
  (`KismetSystemLibrary.K2_SetTimerDelegate` (`|CreateDelegate` :!event `DestroySelf`) (`PaperFlipbookComponent.GetFlipbookLength` (`self.PaperFlipbook`))))

(fn `DestroySelf`
  (`self.K2_DestroyActor`))

(fn `RemoveFB`
  (`PaperFlipbookComponent.PlayFromStart` (`self.Brath`)))

(fn `UserConstructionScript`)
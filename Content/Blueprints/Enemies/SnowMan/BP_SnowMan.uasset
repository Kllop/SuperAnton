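; BP_SnowMan is a snowman enemy that extends a parent enemy's attack and super attack with breath and carrot actors.
; Attack spawns a breath actor above the snowman and plays its flipbook from the start.
; SuperAttck sets a timer shortly before its flipbook ends, while SpawnSuperAttack creates the carrot at the world origin.
; BeginPlay sets a looping timer and a zero-time one-shot, whose bound events are not named.
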(event `self.ReceiveBeginPlay`
  (`parent.ReceiveBeginPlay`)
  (`KismetSystemLibrary.K2_SetTimerDelegate` (`|CreateDelegate` :!event `Event Attack _Event`) 5.0 true)
  (`KismetSystemLibrary.K2_SetTimerDelegate` (`|CreateDelegate` :!event `Event Super Attack_Event`) 0.0))

(fn `Attack`
  (`parent.Attack`)
  (bind _returnvalue (`|SpawnActorFromClass` "/Game/Blueprints/Enemies/SnowMan/BP_SnowMan_Brath.BP_SnowMan_Brath_C" (`KismetMathLibrary.MakeTransform` (+ (`self.K2_GetActorLocation`) (0.0 0.0 150.0))) "AlwaysSpawn" "OverrideRootScale" self null))
  (`PaperFlipbookComponent.PlayFromStart` (`/Game/Blueprints/Enemies/SnowMan/BP_SnowMan_Brath.PaperFlipbook` _returnvalue)))

(fn `SpawnSuperAttack`
  (`|SpawnActorFromClass` "/Game/Blueprints/Enemies/SnowMan/BP_SnowMan_Carrot.BP_SnowMan_Carrot_C" (`KismetMathLibrary.MakeTransform` (0.0 0.0 0.0)) "AlwaysSpawn" "OverrideRootScale" null null))

(fn `SuperAttck`
  (`parent.SuperAttck`)
  (`KismetSystemLibrary.K2_SetTimerDelegate` (`|CreateDelegate` :!event `SpawnSuperAttack`) (- (`PaperFlipbookComponent.GetFlipbookLength` (`self.PaperFlipbook`)) 0.2)))

(fn `UserConstructionScript`
  (`parent.UserConstructionScript`))
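; Test child Blueprint of a boss enemy that exercises an inherited attack event dispatcher.
; On BeginPlay it runs the parent logic, then binds a handler to EventAttack that prints "World".
; Attack, Spawn, Defend, Wait and Death are overridden but only forward to the parent implementations.
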(event `self.ReceiveBeginPlay`
  (`parent.ReceiveBeginPlay`)
  (add `self.Event Attack ` (delegate `Attack _Event_1`)))

(event `Attack _Event_1`
  (`KismetSystemLibrary.PrintString` "World"))

(fn `Attack`
  (`parent.Attack`))

(fn `Death`
  (`parent.Death`))

(fn `Defend`
  (`parent.Defend`))

(fn `Spawn`
  (`parent.Spawn`))

(fn `UserConstructionScript`
  (`parent.UserConstructionScript`))

(fn `Wait`
  (`parent.Wait`))
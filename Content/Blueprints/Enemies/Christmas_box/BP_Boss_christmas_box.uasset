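; Christmas box boss enemy that extends a parent enemy Blueprint with its own projectile attack.
; After the parent BeginPlay and a fixed delay, it fires the attack event once from this graph.
; The Attack override runs the parent logic, then spawns a Christmas box projectile at the attack spawn location, passing on attack damage with no target character.
; Spawn and the construction script only defer to the parent.
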(event `self.ReceiveBeginPlay`
  (`parent.ReceiveBeginPlay`)
  (`KismetSystemLibrary.Delay` 10.0)
  (`self.Event Attack _Event`))

(fn `Attack`
  (`parent.Attack`)
  (bind _returnvalue (`|SpawnActorFromClass` "/Game/Blueprints/Enemies/Christmas_box/BP_Projectile_christmas_box.BP_Projectile_christmas_box_C" (`KismetMathLibrary.MakeTransform` (`self.AttackSpawnLocation`)) "AlwaysSpawn" "OverrideRootScale" null null))
  (set `/Game/Blueprints/Enemies/Christmas_box/BP_Projectile_christmas_box.TargetCharacter` null _returnvalue)
  (set `/Game/Blueprints/Enemies/Christmas_box/BP_Projectile_christmas_box.AttackDamage` (`self.AttackDamage`) _returnvalue)
  (return))

(fn `Spawn`
  (`parent.Spawn`))

(fn `UserConstructionScript`
  (`parent.UserConstructionScript`))
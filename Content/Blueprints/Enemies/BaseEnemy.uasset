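; Base enemy for a side-scroller that climbs or drops between platform levels toward the player and damages them on contact.
; CheckCharacter compares rounded height levels, calling the empty Attack stub when they match.
; CheckPlatform line-traces for a destination platform within level bounds, then a timeline steps the enemy diagonally in Y/Z and rounds its position.
; Box overlap sends DamageMessage; a successful hit disables the box and starts a cooldown timer.
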(event `self.ReceiveBeginPlay`
  (`parent.ReceiveBeginPlay`)
  (`KismetSystemLibrary.K2_SetTimerDelegate` (`|CreateDelegate` :!event `Event Move Enemy`) 1.0 true)
  (`self.Event Move Enemy`))

(event `Event Move Enemy`
  (bind _returnvalue (`GameplayStatics.GetWorldDeltaSeconds`))
  (bind (_step_size_y _step_size_z) (defaults `/Game/Paterns/MatserPlatform/BP_PlatformsParent` "/Game/Paterns/MatserPlatform/BP_PlatformsParent.BP_PlatformsParent_C"))
  (bind _timemove (`self.TimeMove`))
  (bind _returnvalue_2 (/ (* _returnvalue _step_size_y) _timemove))
  (bind _returnvalue_3 (/ (* _returnvalue _step_size_z) _timemove))
  (bind (_vector _current_level) (`self.CheckCharacter`))
  (bind _move (`self.CheckPlatform` _vector _current_level))
  (if _move
    (`Timeline|Move` :!via `PlayFromStart`
      (:`Update`
        (`self.K2_AddActorWorldOffset` (`KismetMathLibrary.MakeVector` 0.0 (select `/Game/DataTables/Enums/E_VectorMoveEnemy` _vector :`NewEnumerator0` _returnvalue_2 :`NewEnumerator1` (* _returnvalue_2 -1.0)) (select `/Game/DataTables/Enums/E_VectorMoveEnemy` _vector :`NewEnumerator0` _returnvalue_3 :`NewEnumerator1` (* _returnvalue_3 -1.0)))))
      (:`Finished`
        (`self.K2_SetActorLocation` (`KismetMathLibrary.MakeVector` (.x (`self.K2_GetActorLocation`)) (`KismetMathLibrary.Conv_IntToDouble` (`KismetMathLibrary.Round` (.y (`self.K2_GetActorLocation`)))) (`KismetMathLibrary.Conv_IntToDouble` (`KismetMathLibrary.Round` (.z (`self.K2_GetActorLocation`))))))))))

(event `self.Box1.OnComponentBeginOverlap`
  (params (OverlappedComponent :type "PrimitiveComponent Object Reference") (OtherActor :type "Actor Object Reference") (OtherComp :type "PrimitiveComponent Object Reference") (OtherBodyIndex :type Integer) (bFromSweep :type Boolean) (SweepResult :type "HitResult Structure (by ref)"))
  (bind _as2dside_scroller_character (cast `/Game/Blueprints/Characters/2DSideScrollerCharacter` OtherActor))
  (`/Engine/EditorBlueprintResources/StandardMacros.IsValid` (`self.LastCharacter`)
    (:`Is Not Valid`
      (bind _newparam (message `/Game/Blueprints/Interfaces/Interface_Damage.Damage` OtherActor (`self.Damage`)))
      (if _newparam
        (set `self.LastCharacter` _as2dside_scroller_character)
        (`KismetSystemLibrary.K2_SetTimerDelegate` (`|CreateDelegate` :!event `RemoveHitCharacter`) 5.0)
        (`PrimitiveComponent.SetCollisionEnabled` (`self.Box1`) "NoCollision")))))

(fn `Attack`)

(fn `CheckCharacter`
  (returns (Vector :type "/Game/DataTables/Enums/E_VectorMoveEnemy Enum") (Current_Level :type Integer))
  (bind _returnvalue (`KismetMathLibrary.Round` (/ (- (.z (`self.K2_GetActorLocation`)) 100.0) (`self.StepSize`))))
  (bind _as2dside_scroller_character (cast `/Game/Blueprints/Characters/2DSideScrollerCharacter` (`GameplayStatics.GetPlayerCharacter` 0))
    (:`then`
      (bind _returnvalue_2 (`GameplayStatics.GetActorOfClass` "/Game/Paterns/MatserPlatform/BP_PlatformsParent.BP_PlatformsParent_C"))
      (`/Engine/EditorBlueprintResources/StandardMacros.IsValid` _returnvalue_2
        (:`Is Valid`
          (bind _output_get (set `self.StepSize` (`/Game/Paterns/MatserPlatform/BP_PlatformsParent.Step_Size_Z` _returnvalue_2)))
          (bind _returnvalue_3 (`KismetMathLibrary.Round` (/ (- (.z (`self.K2_GetActorLocation` _as2dside_scroller_character)) 100.0) _output_get)))
          (if (== _returnvalue _returnvalue_3)
            (`self.Attack`)
            (return "NewEnumerator2" _returnvalue)
            (elif (> (- _returnvalue _returnvalue_3) 0)
              (return "NewEnumerator1" _returnvalue)
              (else
                (return "NewEnumerator0" _returnvalue)))))
        (:`Is Not Valid`
          (return "NewEnumerator2" 0))))
    (:`CastFailed`
      (return "NewEnumerator2" 0))))

(fn `CheckPlatform`
  (params (Vector :type "/Game/DataTables/Enums/E_VectorMoveEnemy Enum" :default "NewEnumerator0") (CurrentLevel :type Integer))
  (returns (Move :type Boolean))
  (bind _returnvalue (- CurrentLevel 1))
  (bind _returnvalue_2 (`self.K2_GetActorLocation`))
  (bind _returnvalue_3 (+ CurrentLevel 1))
  (bind (_step_size_y _step_size_z) (defaults `/Game/Paterns/MatserPlatform/BP_PlatformsParent` "/Game/Paterns/MatserPlatform/BP_PlatformsParent.BP_PlatformsParent_C"))
  (bind (_step_size_y_2 _step_size_z_2) (defaults `/Game/Paterns/MatserPlatform/BP_PlatformsParent` "/Game/Paterns/MatserPlatform/BP_PlatformsParent.BP_PlatformsParent_C"))
  (switch `/Game/DataTables/Enums/E_VectorMoveEnemy` Vector
    (:`NewEnumerator0`
      (if (>= CurrentLevel 2)
        (return false)
        (else
          _)))
    (:`NewEnumerator1`
      (if (<= CurrentLevel 0)
        (return false)
        (else
          _)))
    (:`NewEnumerator2`
      (return false)))
  (bind (_outhit _returnvalue_4) (`KismetSystemLibrary.LineTraceSingleForObjects` :`Start` _returnvalue_2 :`End` (`KismetMathLibrary.MakeVector` (.x _returnvalue_2) (select `/Game/DataTables/Enums/E_VectorMoveEnemy` Vector :`NewEnumerator0` (* _returnvalue_3 _step_size_y_2) :`NewEnumerator1` (* _returnvalue _step_size_y)) (select `/Game/DataTables/Enums/E_VectorMoveEnemy` Vector :`NewEnumerator0` (- (* _returnvalue_3 _step_size_z_2) 10.0) :`NewEnumerator1` (- (* _returnvalue _step_size_z) 10.0))) :`ObjectTypes` (`|MakeArray` "ObjectTypeQuery6" :!type "EObjectTypeQuery Enum") :`DrawTime` 1.0))
  (if _returnvalue_4
    (return true)
    (else
      (return false))))

(fn `RemoveHitCharacter`
  (set `self.LastCharacter` null)
  (`PrimitiveComponent.SetCollisionEnabled` (`self.Box1`) "QueryOnly"))

(fn `UserConstructionScript`
  (`parent.UserConstructionScript`))